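; Sun controller that drives a directional light's rotation from a normalized time of day.
; On BeginPlay it uses the assigned light, or warns and searches the level for directional lights.
; Set and Increment functions clamp the time and set a goal rotation, which Tick eases toward over the blend time.
; TimeToSunRotation supplies the rotations, though its only visible node, a morning-to-sunset lerp, is unused.
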(event Custom|Begin%20Moving%20sun
  ;[0 0.5781 1] Begin moving sun
  (Variables|Default|SetStart%20rotation (Transformation|GetWorldRotation (Variables|Default|GetSunlight%20Ref)))
  (Variables|Default|SetMoveTimePassed 0.0)
  (Variables|Default|SetMoving%20sun? true))

(event EventBeginPlay
  ;[0.8516 0 1] Get light ref at start of game
  (Utilities|IsValid (Variables|Default|GetSun%20Ref)
    (:Is%20Valid
      (bind _output_get (Variables|Default|SetSunlight%20Ref (Variables|/Script/Engine.Light|GetLightComponent (Variables|Default|GetSun%20Ref)) :!label _label))
      ;[0.7578 1 0] Initialize sun from time of day
      (Transformation|SetWorldRotation _output_get (Utilities|TimetoSunRotation (Variables|Default|GetTimeOfDay)) false false))
    (:Is%20Not%20Valid
      (Development|PrintString "WARNING: Directional light not set in suntime controller. Automatically setting...")
      (bind _outactors (Actor|GetAllActorsOfClass "/Script/Engine.DirectionalLight"))
      (for _array_element _outactors
        (Variables|Default|SetSun%20Ref _array_element)
        (goto _label)))))

(event EventTick
  (params (DeltaSeconds :type Float%20%28single-precision%29))
  ;[0.5 1 0] Ease sun to desired rotation over ease time
  (if (Variables|Default|GetMoving%20sun?)
    (Variables|Default|SetMoveTimePassed (+ (Variables|Default|GetMoveTimePassed) DeltaSeconds))
    (Transformation|SetWorldRotation (Variables|Default|GetSunlight%20Ref) (Math|Interpolation|Ease "EaseInOut" (/ (Variables|Default|GetMoveTimePassed) (Variables|Default|GetEase%20time)) (Variables|Default|GetStart%20rotation) (Variables|Default|GetRotationGoal) true) false false)
    (if (> (Variables|Default|GetMoveTimePassed) (Variables|Default|GetEase%20time))
      (Variables|Default|SetMoving%20sun? false))))

(fn ConstructionScript)

(fn SetTimeOfDay
  (params (new%20time :type Float%20%28single-precision%29) (Blend%20Time :type Float%20%28single-precision%29))
  (bind _returnvalue (Math|Float|Clamp(Float) new%20time))
  (Variables|Default|SetEase%20time Blend%20Time)
  (Variables|Default|SetTimeOfDay _returnvalue)
  (Variables|Default|SetRotationGoal (Utilities|TimetoSunRotation _returnvalue))
  (CallFunction|BeginMovingSun))

(fn IncrementTimeOfDay
  (params (Time%20offset :type Float%20%28single-precision%29) (Blend%20Time :type Float%20%28single-precision%29))
  (Variables|Default|SetEase%20time Blend%20Time)
  (bind _output_get (Variables|Default|SetTimeOfDay (Math|Float|Clamp(Float) (+ Time%20offset (Variables|Default|GetTimeOfDay)))))
  (Variables|Default|SetRotationGoal (Utilities|TimetoSunRotation _output_get))
  (CallFunction|BeginMovingSun))