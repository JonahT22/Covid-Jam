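; In-world to-do list actor that shows a checklist and up to two sticky notes through widget components.
; On BeginPlay it caches the WB_TodoList widget and loads the first list with an item already checked off.
; Events switch between two predefined lists, check off items, and reveal or check off sticky notes by number.
; Revealing a sticky note sets its WB_StickyNote text and unhides its component.
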(event Custom|Set%20TodoList
  (params (List%20Number :type Integer))
  (bind _todo_list_widget (Variables|Default|GetTodo%20List%20Widget))
  ;[0 0.5312 1] Initialize new todo list
  (switch int List%20Number
    (:Default
      (Development|PrintString "ERROR: Invalid todo list" :!label _label))
    (:0
      (goto _label))
    (:1
      (Default|FillTodoList _todo_list_widget (Variables|Default|GetTodoList%201))
      (Default|CheckOffItem _todo_list_widget 1) ; start with lunch checked off
    )
    (:2
      (Default|FillTodoList _todo_list_widget (Variables|Default|GetTodoList%202)))))

(event Custom|Check%20off%20item
  (params (Item%20index :type Integer))
  ;[0 0.4141 1] Check off tasks
  (Default|CheckOffItem (Variables|Default|GetTodo%20List%20Widget) Item%20index))

(event Custom|Reveal%20Sticky%201
  ;[1 0 0.2812] Reveal sticky notes
  (bind _aswb_sticky_note (Utilities|Casting|CastToWB_StickyNote (UserInterface|GetUserWidgetObject (Variables|Default|GetSticky%201))))
  (Default|SetStickyText _aswb_sticky_note (Variables|Default|GetSticky%201%20text))
  (Development|SetHiddeninGame (Variables|Default|GetSticky%201) false false))

(event Custom|Reveal%20Sticky%202
  ;[1 0 0.2812] Reveal sticky notes
  (bind _aswb_sticky_note (Utilities|Casting|CastToWB_StickyNote (UserInterface|GetUserWidgetObject (Variables|Default|GetSticky%202))))
  (Default|SetStickyText _aswb_sticky_note (Variables|Default|GetSticky%202%20text))
  (Development|SetHiddeninGame (Variables|Default|GetSticky%202) false false))

(event Custom|Add%20Sticky%20note
  (params (Sticky%20number :type Integer))
  ;[1 0.5859 0] choose a sticky note to reveal
  (switch int Sticky%20number
    (:Default
      (Development|PrintString "ERROR: Invalid sticky note index added to todo list" :!label _label))
    (:0
      (goto _label))
    (:1
      (CallFunction|RevealSticky1))
    (:2
      (CallFunction|RevealSticky2))))

(event Custom|CheckOffSticky
  (params (Sticky# :type Integer))
  (switch int Sticky#
    (:1
      (bind _aswb_sticky_note (Utilities|Casting|CastToWB_StickyNote (UserInterface|GetUserWidgetObject (Variables|Default|GetSticky%201))))
      (Default|CheckOff _aswb_sticky_note (Variables|Default|GetSticky%201%20text)))
    (:2
      (bind _aswb_sticky_note_2 (Utilities|Casting|CastToWB_StickyNote (UserInterface|GetUserWidgetObject (Variables|Default|GetSticky%202))))
      (Default|CheckOff _aswb_sticky_note_2 (Variables|Default|GetSticky%202%20text)))))

(event EventBeginPlay
  ;[1 0 0.7031] Begin play
  (bind _aswb_todo_list (Utilities|Casting|CastToWB_TodoList (UserInterface|GetUserWidgetObject (Variables|Default|GetListWidget))))
  (Variables|Default|SetTodo%20List%20Widget _aswb_todo_list)
  (CallFunction|SetTodoList 1))

(fn ConstructionScript)