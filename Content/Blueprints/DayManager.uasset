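; Level manager that scripts the game's two-day story, sequencing tutorial and morning dialogue, to-do lists and which interactables are active.
; BeginPlay validates its references and starts day 1, then externally callable stage events activate objects such as chess, sofa, computer and soup.
; Ending day 1 resets the sun and phone/thought UI, then teleports the player to a day 2 spawn.
; Ending day 2 shows the end screen and returns to the main menu.
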(event Custom|Begin%20Day%201
  (bind _io_chess (Variables|Default|GetIO_Chess))
  ;[1 1 1] Begin day 1
  (Variables|/Game/Blueprints/Char_CovidCharacter.Char_CovidCharacter_C|SetCanMove? (Variables|Default|GetPlayerCharacter) false)
  (Default|AddDialoguetoQueue (Variables|Default|GetDialogueController) "/Game/Blueprints/DialogueInteractions/ConversationSheets/Dialogue_Interactions_-_Tutorial01.Dialogue_Interactions_-_Tutorial01")
  (Default|SetTodoList (Variables|Default|GetTodoList) 1)
  (Utilities|FlowControl|Delay 2.0)
  (Default|BecomeActive _io_chess)
  (Default|SetDay _io_chess 1)
  (bind _outactors (Actor|GetAllActorsOfClass "/Game/Blueprints/InteractableObjects/InteractableObject.InteractableObject_C"))
  (for _array_element _outactors
    (Variables|/Game/Blueprints/InteractableObjects/InteractableObject.InteractableObject_C|SetDay%201? _array_element true)))

(event Custom|Begin%20Day%202
  (bind _day2spawn (Variables|Default|GetDay2Spawn))
  (bind _returnvalue (Transformation|GetActorTransform _day2spawn))
  ;[1 1 1] Begin day 2
  (Transformation|SetActorLocationAndRotation (Variables|Default|GetPlayerCharacter) (.location _returnvalue) (.rotation _returnvalue) false true)
  (Default|SetDay (Variables|Default|GetIO_Chess) 2)
  (bind _outactors (Actor|GetAllActorsOfClass "/Game/Blueprints/InteractableObjects/InteractableObject.InteractableObject_C"))
  (for _array_element _outactors
    (Variables|/Game/Blueprints/InteractableObjects/InteractableObject.InteractableObject_C|SetDay%201? _array_element false))
  (Variables|/Game/Blueprints/Char_CovidCharacter.Char_CovidCharacter_C|SetCanMove? (Variables|Default|GetPlayerCharacter) false)
  (Default|BecomeActive (Variables|Default|GetIO_CleaningSupplies))
  (Default|SetTodoList (Variables|Default|GetTodoList) 2)
  (Utilities|FlowControl|Delay 0.5)
  (Default|FadefromBlack (Variables|Default|GetDialogueController))
  (Utilities|FlowControl|Delay 2.0)
  (Variables|/Game/Blueprints/Char_CovidCharacter.Char_CovidCharacter_C|SetCanMove? (Variables|Default|GetPlayerCharacter) true)
  (Default|AddDialoguetoQueue (Variables|Default|GetDialogueController) "/Game/Blueprints/DialogueInteractions/ConversationSheets/Dialogue_Interactions_-_Morning.Dialogue_Interactions_-_Morning"))

(event Custom|End%20Day%201
  (bind _playercontroller (Variables|Default|GetPlayerController))
  (bind _gameplay_ui (Variables|/Game/Blueprints/PC_Covid.PC_Covid_C|GetGameplay%20UI _playercontroller))
  ;[1 1 1] End day 1
  (Default|SetTimetoMorning (Variables|Default|GetSunTimeController))
  (Default|ClearBox (Variables|/Game/UI/WB_GameplayUI.WB_GameplayUI_C|GetPhoneScrollBox _gameplay_ui))
  (Default|ClearBox (Variables|/Game/UI/WB_GameplayUI.WB_GameplayUI_C|GetThoughtsScrollBox _gameplay_ui))
  (CallFunction|BeginDay2))

(event Custom|End%20Day%202
  (bind _playercharacter (Variables|Default|GetPlayerCharacter))
  (bind _playercontroller (Variables|Default|GetPlayerController))
  ;[1 1 1] End day 2
  (Variables|/Game/Blueprints/Char_CovidCharacter.Char_CovidCharacter_C|SetCanMove? _playercharacter false)
  (Variables|/Game/Blueprints/Char_CovidCharacter.Char_CovidCharacter_C|SetCanInteract? _playercharacter false)
  (Default|EndMusic _playercontroller)
  (Default|EndOfGame (Variables|/Game/Blueprints/PC_Covid.PC_Covid_C|GetGameplay%20UI _playercontroller))
  (Utilities|FlowControl|Delay 15.0)
  (Game|OpenLevel(byName) "MainMenu"))

(event Custom|Day1%20Part3
  ;[1 1 1] Enable cleaning supplies day 1
  (Default|BecomeActive (Variables|Default|GetIO_CleaningSupplies)))

(event Custom|Day1%20Part2
  ;[1 1 1] Let player move day 1
  (Variables|/Game/Blueprints/Char_CovidCharacter.Char_CovidCharacter_C|SetCanMove? (Variables|Default|GetPlayerCharacter) true)
  (Default|BecomeActive (Variables|Default|GetIO_Sofa))
  (Default|BecomeActive (Variables|Default|GetIO_Dishes))
  (Default|BecomeActive (Variables|Default|GetIO_Chess))
  (Default|BecomeActive (Variables|Default|GetIO_Door)))

(event Custom|Day%202%20-%20Activate%20computer
  ;[1 1 1] During day 2
  (Default|BecomeActive (Variables|Default|GetIO_Computer)))

(event Custom|Day%202%20-%20Activate%20Soup
  ;[1 1 1] During day 2
  (Default|BecomeActive (Variables|Default|GetIO_SoupPot)))

(event Custom|Day%202%20-%20Activate%20Chess
  ;[1 1 1] During day 2
  (Default|BecomeActive (Variables|Default|GetIO_Chess)))

(event EventBeginPlay
  (bind _aspc_covid (Utilities|Casting|CastToPC_Covid (Game|GetPlayerController 0)))
  (Variables|Default|SetPlayerController _aspc_covid)
  (bind _aschar_covid_character (Utilities|Casting|CastToChar_CovidCharacter (Game|GetPlayerCharacter 0)))
  (Variables|Default|SetPlayerCharacter _aschar_covid_character)
  (if (Math|Boolean|ANDBoolean (Utilities|IsValid (Variables|Default|GetDay2Spawn)) (Utilities|IsValid (Variables|Default|GetIO_Chess)) (Utilities|IsValid (Variables|Default|GetDialogueController)) (Utilities|IsValid (Variables|Default|GetIO_Sofa)) (Utilities|IsValid (Variables|Default|GetIO_Dishes)) (Utilities|IsValid (Variables|Default|GetIO_Door)) (Utilities|IsValid (Variables|Default|GetIO_CleaningSupplies)) (Utilities|IsValid (Variables|Default|GetIO_Computer)) (Utilities|IsValid (Variables|Default|GetIO_SoupPot)) (Utilities|IsValid (Variables|Default|GetSunTimeController)) (Utilities|IsValid (Variables|Default|GetTodoList)))
    (CallFunction|BeginDay1)
    (else
      (Development|PrintString "ERROR: MISSING REFERENCES IN DAYMANAGER BP" true true "(R=0.000000,G=0.660000,B=1.000000,A=1.000000)" 2e+01))))

(fn ConstructionScript)