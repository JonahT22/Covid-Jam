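; DC_TestChild is a test child dialogue interaction Blueprint that animates the level's directional light to a new rotation, moving the sun.
; Its CustomEvent1 loops over all DirectionalLight actors, keeps the last one's light component, then records its starting rotation and resets the timer.
; Tick then eases the light in and out toward RotationGoal over EaseTime, clearing the moving flag afterward.
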(event Custom|Begin%20moving%20sun
  ;[1 0 0.7969] Begin moving sun
  (Variables|Default|SetStart%20rotation (Transformation|GetWorldRotation (Variables|Default|GetSunlight)))
  (Variables|Default|SetTime%20passed 0.0)
  (Variables|Default|SetMoving%20sun? true))

(event EventBeginPlay
  (|CallParentFunction) ; This node is disabled and will not be called.\nDrag off pins to build functionality.
)

(event Collision|EventActorBeginOverlap
  (params (OtherActor :type Actor%20Object%20Reference)))

(event EventTick
  (params (DeltaSeconds :type Float%20%28single-precision%29))
  (|CallParentFunction DeltaSeconds)
  ;[1 0 0.3281] Ease to sun desired rotation over ease time
  (if (Variables|Default|GetMoving%20sun?)
    (Variables|Default|SetTime%20passed (+ (Variables|Default|GetTime%20passed) DeltaSeconds))
    (Transformation|SetWorldRotation (Variables|Default|GetSunlight) (Math|Interpolation|Ease "EaseInOut" (/ (Variables|Default|GetTime%20passed) (Variables|Default|GetEase%20time)) (Variables|Default|GetStart%20rotation) (Variables|Default|GetRotationGoal) true) false false)
    (if (> (Variables|Default|GetTime%20passed) (Variables|Default|GetEase%20time))
      (Variables|Default|SetMoving%20sun? false))))

(event EventCustomEvent1
  ;[0.3359 1 0] Custom event 1: move sun
  (bind _outactors (Actor|GetAllActorsOfClass "/Script/Engine.DirectionalLight"))
  (for _array_element _outactors
    (Variables|Default|SetSunlight (Variables|/Script/Engine.Light|GetLightComponent _array_element)))
  (CallFunction|BeginMovingSun))

(fn ConstructionScript
  (|CallParentFunction))