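; Base interactable object that shows an interaction prompt while the player character overlaps its capsule.
; Entering the capsule while the object is active sets the interactable flag and reveals the text widget; leaving clears both.
; InteractionEvent, meant to be overridden in child Blueprints, activates the assigned DialogueTrigger by default or prints an error if it is invalid.
; The construction script copies InteractionText into the prompt widget.
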(event OnComponentBeginOverlap(Capsule)
  (params (OverlappedComponent :type Primitive%20Component%20Object%20Reference) (OtherActor :type Actor%20Object%20Reference) (OtherComp :type Primitive%20Component%20Object%20Reference) (OtherBodyIndex :type Integer) (bFromSweep :type Boolean) (SweepResult :type Hit%20Result%20Structure%20%28by%20ref%29))
  ;[0 1 0.8594] Begin/End overlap
  (if (Variables|Default|GetAm%20Active?)
    (if (== OtherActor (Variables|Default|GetPlayerCharacter))
      (Variables|Default|SetAm%20Interactable? true)
      (Development|SetHiddeninGame (Variables|Default|GetInteract%20Text) false false))))

(event OnComponentEndOverlap(Capsule)
  (params (OverlappedComponent :type Primitive%20Component%20Object%20Reference) (OtherActor :type Actor%20Object%20Reference) (OtherComp :type Primitive%20Component%20Object%20Reference) (OtherBodyIndex :type Integer))
  ;[0 1 0.8594] Begin/End overlap
  (if (== OtherActor (Variables|Default|GetPlayerCharacter))
    (Variables|Default|SetAm%20Interactable? false)
    (Development|SetHiddeninGame (Variables|Default|GetInteract%20Text) true false)))

(event Custom|Interaction%20Event
  (bind _dialoguetrigger (Variables|Default|GetDialogueTrigger))
  (Utilities|IsValid _dialoguetrigger
    (:Is%20Valid
      (Default|ActivateDialogueController _dialoguetrigger))
    (:Is%20Not%20Valid
      (Development|PrintString "ERROR: Invalid dialogue trigger in interactable object"))))

(event EventBeginPlay
  ;[1 0 0.375] get player character at start of game
  (bind _aschar_covid_character (Utilities|Casting|CastToChar_CovidCharacter (Game|GetPlayerCharacter 0)))
  (Variables|Default|SetPlayerCharacter _aschar_covid_character)
  (Variables|Default|SetPlayer%20Camera (Variables|/Game/Blueprints/Char_CovidCharacter.Char_CovidCharacter_C|GetFirstPersonCamera _aschar_covid_character)))

(fn ConstructionScript
  (CallFunction|SetInteractText))

(fn SetInteractText
  (bind _asinteractable_object_text (Utilities|Casting|CastToInteractableObjectText (UserInterface|GetUserWidgetObject (Variables|Default|GetInteract%20Text))))
  (Rendering|Components|TextRender|SetText (Variables|/Game/Blueprints/InteractableObjectText.InteractableObjectText_C|GetInteractionText _asinteractable_object_text) (Variables|Default|GetInteractionText)))