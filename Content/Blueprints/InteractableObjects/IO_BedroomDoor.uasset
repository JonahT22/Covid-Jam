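; Bedroom door interactable that serves as a soup delivery point rather than an openable door.
; Interaction triggers DeliverSoup, which prints a debug message, plays a knocking sound at the mouse-over box and queues the "Final Moments" interaction dialogue on the dialogue controller.
; A timeline-driven open/close toggle that yaws the mesh remains in the graph but is disconnected and never runs.
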(event Custom|DeliverSoup
  (Development|PrintString "SOUP DELIVERED")
  (Audio|PlaySoundatLocation "/Game/Audio/Door_Kocking.Door_Kocking" (Transformation|GetWorldLocation (Variables|Default|GetMouseOverBox)) "0, 0, 0" 1.0 1.0 0.0 "/Game/Audio/DefaultAttenuation.DefaultAttenuation" 0 0)
  (Default|AddDialoguetoQueue (Variables|Default|GetDialogueController%20Ref) "/Game/Blueprints/DialogueInteractions/ConversationSheets/Dialogue_Interactions_-_Final_Moments.Dialogue_Interactions_-_Final_Moments"))

(event EventBeginPlay
  (|CallParentFunction) ; This node is disabled and will not be called.\nDrag off pins to build functionality.
)

(event Collision|EventActorBeginOverlap
  (params (OtherActor :type Actor%20Object%20Reference)))

(event EventTick
  (params (DeltaSeconds :type Float%20%28single-precision%29)))

(event EventInteractionEvent
  (CallFunction|DeliverSoup))

(fn ConstructionScript
  (|CallParentFunction))