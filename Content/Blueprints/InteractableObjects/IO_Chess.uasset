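; Interactable chess board that plays out a scripted game across days, starting with a tutorial move.
; Each interaction advances a counter that plays a tap sound, queues dialogue and snaps pieces to hard-coded relative positions, deactivating the board after certain moves.
; SetDay replays the first day's moves on later days to restore the board.
; The final move checks off a to-do item and triggers the Day Manager's soup event.
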(event Custom|ChessPlay
  (params (TimesCalled :type Integer))
  (Audio|PlaySoundatLocation "/Game/Audio/Chess_Tap.Chess_Tap" "0, 0, 0" "0, 0, 0" 1.0 1.0 0.0 0 0 0)
  (if (== (Variables|Default|GetTimesCalled) -1)
    (CallFunction|ChessTutorialMove)
    (else
      (CallFunction|SendDialogueSheettoController TimesCalled)
      (switch int TimesCalled
        (:Default
          (Development|PrintString "ERROR: Invalid chess move index"))
        (:0
          (CallFunction|Chess1-1)
          (CallFunction|Chess1-2))
        (:1
          (CallFunction|Chess1-3)
          (CallFunction|Chess1-4))
        (:2
          (CallFunction|Chess1-5)
          (if (Variables|Default|GetisDay1)
            (CallFunction|BecomeInactive)
            (else
              (CallFunction|BecomeInactive)
              (Utilities|FlowControl|Delay 5.0)
              (CallFunction|BecomeActive))))
        (:3
          (CallFunction|Chess2-1))
        (:4
          (CallFunction|Chess2-2))
        (:5
          (CallFunction|Chess2-3)
          (CallFunction|BecomeInactive))))))

(event Custom|ChessTutorialMove
  (Default|AddDialoguetoQueue (Variables|Default|GetDialogueController%20Ref) "/Game/Blueprints/DialogueInteractions/ConversationSheets/Dialogue_Interactions_-_Tutorial02.Dialogue_Interactions_-_Tutorial02")
  (Transformation|SetRelativeLocation (Variables|Default|GetBlack_Queen) "3.900000,-22.700001,8.820000" false false)
  (Transformation|SetRelativeLocation (Variables|Default|GetWhite_Pawn06) "12.800000,4.300000,6.480000" false false)
  (Transformation|SetRelativeLocation (Variables|Default|GetBlack_Bishop02) "21.200001,5.300000,8.290000" false false)
  (CallFunction|BecomeInactive))

(event Custom|SetDay
  (params (Day :type Integer))
  (if (== Day 1)
    (Variables|Default|SetisDay1 true)
    (else
      (Variables|Default|SetisDay1 false)
      (CallFunction|Chess1-1)
      (CallFunction|Chess1-2)
      (CallFunction|Chess1-3)
      (CallFunction|Chess1-4)
      (CallFunction|Chess1-5)
      (Variables|Default|SetTimesCalled 3))))

(event Custom|Chess2-1
  ;[0 1 0.2031] Chess moves
  (Transformation|SetRelativeLocation (Variables|Default|GetWhite_Pawn07) "13.000000,4.260000,6.480000" false false)
  (Transformation|SetRelativeLocation (Variables|Default|GetBlack_Knight) "-57.500000,25.299999,5.680000" false false)
  (CallFunction|BecomeInactive))

(event Custom|Chess2-2
  ;[0 1 0.2031] Chess moves
  (Transformation|SetRelativeLocation (Variables|Default|GetBlack_Queen) "21.400000,-22.299999,8.820000" false false)
  (Transformation|SetRelativeLocation (Variables|Default|GetWhite_King) "21.900000,21.700001,10.160000" false false)
  (CallFunction|BecomeInactive))

(event Custom|Chess2-3
  ;[0 1 0.2031] Chess moves
  (Transformation|SetRelativeLocation (Variables|Default|GetBlack_Bishop02) "21.400000,5.100000,8.290000" false false)
  (CallFunction|BecomeInactive)
  (Default|CheckOffItem (Variables|Default|GetTodo%20List%20Ref) 3)
  (Default|Day2-ActivateSoup (Variables|Default|GetDayManager%20Ref)))

(event Custom|Chess1-1
  ;[0 1 0.2031] Chess moves
  (Transformation|SetRelativeLocation (Variables|Default|GetWhite_Queen) "5.000000,31.100000,8.970000" false false)
  (Transformation|SetRelativeLocation (Variables|Default|GetBlack_Pawn05) "-50.000000,11.600000,4.500000" false false)
  (Transformation|SetRelativeLocation (Variables|Default|GetWhite_Rook02) "12.500000,3.900000,6.770000" false false))

(event Custom|Chess1-2
  ;[0 1 0.2031] Chess moves
  (Transformation|SetRelativeLocation (Variables|Default|GetBlack_Rook02) "-49.000000,3.500000,4.900000" false false)
  (Transformation|SetRelativeLocation (Variables|Default|GetWhite_Bishop01) "46.700001,-21.500000,5.400000" false false)
  (Transformation|SetRelativeLocation (Variables|Default|GetWhite_Pawn08) "22.200001,-3.940000,6.480000" false false)
  (CallFunction|BecomeInactive))

(event Custom|Chess1-3
  ;[0 1 0.2031] Chess moves
  (Transformation|SetRelativeLocation (Variables|Default|GetBlack_Queen) "4.000000,-4.700000,8.800000" false false)
  (Transformation|SetRelativeLocation (Variables|Default|GetWhite_Queen) "21.600000,12.600000,8.960000" false false))

(event Custom|Chess1-4
  ;[0 1 0.2031] Chess moves
  (Transformation|SetRelativeLocation (Variables|Default|GetBlack_Queen) "0, 0, 0" false false)
  (Transformation|SetRelativeLocation (Variables|Default|GetWhite_Rook01) "12.500000,30.799999,6.800000" false false)
  (CallFunction|BecomeInactive))

(event Custom|Chess1-5
  ;[0 1 0.2031] Chess moves
  (Transformation|SetRelativeLocation (Variables|Default|GetBlack_Rook01) "-4.600000,-31.600000,6.950000" false false)
  (Transformation|SetRelativeLocation (Variables|Default|GetBlack_King) "-13.600000,-30.600000,10.200000" false false)
  (Transformation|SetRelativeLocation (Variables|Default|GetWhite_Queen) "30.200001,20.900000,8.960000" false false)
  (Transformation|SetRelativeLocation (Variables|Default|GetBlack_Knight) "30.500000,-4.300000,7.760000" false false))

(event EventBeginPlay
  (|CallParentFunction)
  (Variables|Default|SetTimesCalled -2))

(event Collision|EventActorBeginOverlap
  (params (OtherActor :type Actor%20Object%20Reference)))

(event EventTick
  (params (DeltaSeconds :type Float%20%28single-precision%29)))

(event EventInteractionEvent
  (bind _output_get (Variables|Default|SetTimesCalled (+ (Variables|Default|GetTimesCalled) 1)))
  (CallFunction|ChessPlay _output_get))

(fn ConstructionScript
  (|CallParentFunction))