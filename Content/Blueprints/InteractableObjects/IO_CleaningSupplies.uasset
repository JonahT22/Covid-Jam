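; Interactable cleaning supplies that the player uses to disinfect, completing a to-do list task.
; Interaction deactivates the object, checks off its sticky note and sends dialogue sheets to the controller, branching on Day1.
; When Day1 is false, it sends the dinner prompt and starts the Day Manager's Day 2 part 2.
; While active and interactable, it shows interact text and outlines its meshes through custom depth.
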(event Custom|Disinfect
  (CallFunction|BecomeInactive)
  (if (Variables|Default|GetDay1?)
    (CallFunction|SendDialogueSheettoController)
    (CallFunction|SendDialogueSheettoController 1)
    (else
      (CallFunction|SendDialogueSheettoController 2) ; Send dinner prompt
      (Default|Day2Part2 (Variables|Default|GetDayManager%20Ref)))))

(event EventBeginPlay
  (|CallParentFunction) ; This node is disabled and will not be called.\nDrag off pins to build functionality.
)

(event Collision|EventActorBeginOverlap
  (params (OtherActor :type Actor%20Object%20Reference)))

(event EventTick
  (params (DeltaSeconds :type Float%20%28single-precision%29)))

(event EventInteractionEvent
  (CallFunction|Disinfect)
  (CallFunction|CheckOffSticky 2))

(fn ConstructionScript
  (|CallParentFunction))

(fn ChangeInteractable
  (params (Interactable? :type Boolean))
  (if (Variables|Default|GetAm%20Active?)
    (if Interactable?
      (Development|SetHiddeninGame (Variables|Default|GetInteract%20Text) false false)
      (Variables|Default|SetAm%20Interactable? true)
      (Rendering|SetRenderCustomDepth (Variables|Character|GetMesh) true)
      (else
        (Development|SetHiddeninGame (Variables|Default|GetInteract%20Text) true false)
        (Variables|Default|SetAm%20Interactable? false)
        (Rendering|SetRenderCustomDepth (Variables|Character|GetMesh) false)))
    (else
      (Rendering|SetRenderCustomDepth (Variables|Character|GetMesh) false))))

(fn CheckOffSticky
  (params (sticky%20number :type Integer))
  (Default|CheckOffSticky (Variables|Default|GetTodo%20List%20Ref) sticky%20number))