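; Interactable coffee mug that toggles between empty and full, starting empty.
; Each interaction runs ChangeState, which flips IsFull, shows or hides the particle effect and reapplies the same mug mesh in both states.
; Filling makes the mug active and every IO_CoffeePot in the level inactive; emptying reverses both, with pots found through GetAllActorsOfClass.
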(event Custom|ChangeState
  (bind _particlesystem (Variables|Default|GetParticleSystem))
  (bind _mesh (Variables|Character|GetMesh))
  (if (Variables|Default|GetisFull)
    (Components|StaticMesh|SetStaticMesh _mesh "/Game/Geometry/Meshes/ALL_mug.ALL_mug")
    (Rendering|SetVisibility _particlesystem false false)
    (CallFunction|BecomeInactive)
    (Variables|Default|SetisFull false)
    (bind _outactors (Actor|GetAllActorsOfClass "/Game/Blueprints/InteractableObjects/IO_CoffeePot.IO_CoffeePot_C"))
    (Default|BecomeActive _outactors)
    (else
      (Components|StaticMesh|SetStaticMesh _mesh "/Game/Geometry/Meshes/ALL_mug.ALL_mug")
      (Rendering|SetVisibility _particlesystem true false)
      (CallFunction|BecomeActive)
      (Variables|Default|SetisFull true)
      (bind _outactors_2 (Actor|GetAllActorsOfClass "/Game/Blueprints/InteractableObjects/IO_CoffeePot.IO_CoffeePot_C"))
      (Default|BecomeInactive _outactors_2))))

(event EventBeginPlay
  (|CallParentFunction)
  (Variables|Default|SetisFull false))

(event Collision|EventActorBeginOverlap
  (params (OtherActor :type Actor%20Object%20Reference)))

(event EventTick
  (params (DeltaSeconds :type Float%20%28single-precision%29)))

(event EventInteractionEvent
  (CallFunction|ChangeState))

(fn ConstructionScript
  (|CallParentFunction))