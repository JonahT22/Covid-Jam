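; Interactable computer object that plays a filing-for-unemployment dialogue and displays text on its screen.
; Its interaction event queues that dialogue through the dialogue controller.
; A separate AddComputertext event passes new text to the ComputerScreen widget's scroll box via the ComputerText component, then sets the object inactive.
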(event Custom|Add%20Computer%20text
  (params (New%20Text :type Text))
  ;[0.1719 0 1] Add text to widget
  (bind _ascomputer_screen (Utilities|Casting|CastToComputerScreen (UserInterface|GetUserWidgetObject (Variables|Default|GetComputerText))))
  (Default|AddTexttoScreenScrollBox _ascomputer_screen New%20Text)
  (CallFunction|BecomeInactive))

(event EventBeginPlay
  (|CallParentFunction) ; This node is disabled and will not be called.\nDrag off pins to build functionality.
)

(event Collision|EventActorBeginOverlap
  (params (OtherActor :type Actor%20Object%20Reference)))

(event EventTick
  (params (DeltaSeconds :type Float%20%28single-precision%29)))

(event EventInteractionEvent
  (Default|AddDialoguetoQueue (Variables|Default|GetDialogueController%20Ref) "/Game/Blueprints/DialogueInteractions/ConversationSheets/Dialogue_Interactions_-_Filing_for_Unemployment.Dialogue_Interactions_-_Filing_for_Unemployment"))

(fn ConstructionScript
  (|CallParentFunction))