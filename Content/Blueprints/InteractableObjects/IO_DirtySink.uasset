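; Interactable dirty sink full of dishes that the player cleans as a Day 1 task.
; Interaction plays a clacking sound, advances the DayManager to Day 1 Part 3, adds a bathroom sticky note and destroys the actor, alongside checking off its task and sending dialogue.
; While active, toggling interactability shows or hides the prompt text and switches custom depth rendering on the main mesh and dish pieces.
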(event Custom|CleanSink
  (bind _daymanager_ref (Variables|Default|GetDayManager%20Ref))
  (Audio|PlaySoundatLocation "/Game/Audio/Bowls_Clacking.Bowls_Clacking" "0, 0, 0" "0, 0, 0" 1.0 1.0 0.0 0 0 0)
  (Default|Day1Part3 _daymanager_ref)
  (Default|AddStickyNoteforBathroom (Variables|/Game/Blueprints/DayManager.DayManager_C|GetDiologueController _daymanager_ref))
  (Actor|DestroyActor))

(event EventBeginPlay
  (|CallParentFunction))

(event Collision|EventActorBeginOverlap
  (params (OtherActor :type Actor%20Object%20Reference)))

(event EventTick
  (params (DeltaSeconds :type Float%20%28single-precision%29)))

(event EventInteractionEvent
  (CallFunction|CleanSink)
  (CallFunction|CheckOffTask 2)
  (CallFunction|SendDialogueSheettoController))

(fn ConstructionScript
  (|CallParentFunction))

(fn ChangeInteractable
  (params (Interactable? :type Boolean))
  (if (Variables|Default|GetAm%20Active?)
    (if Interactable?
      (Development|SetHiddeninGame (Variables|Default|GetInteract%20Text) false false)
      (Variables|Default|SetAm%20Interactable? true)
      (Rendering|SetRenderCustomDepth (Variables|Character|GetMesh) true)
      (else
        (Development|SetHiddeninGame (Variables|Default|GetInteract%20Text) true false)
        (Variables|Default|SetAm%20Interactable? false)
        (Rendering|SetRenderCustomDepth (Variables|Character|GetMesh) false)))))