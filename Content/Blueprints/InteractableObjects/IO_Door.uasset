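; Interactable door that starts with its mesh swung open at a fixed yaw and toggles on each InteractionEvent.
; The OpenDoor timeline drives the mesh's relative yaw, scaled by OpenAngle.
; The first interaction reverses the timeline from its end, and later ones alternate play and reverse through the Open flag.
; Every interaction plays the Door_Open sound at world origin rather than at the door.
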(event EventBeginPlay
  (|CallParentFunction)
  (Transformation|SetRelativeRotation (Variables|Character|GetMesh) (Math|Rotator|MakeRotator 0.0 0.0 1e+02) false false))

(event Collision|EventActorBeginOverlap
  (params (OtherActor :type Actor%20Object%20Reference)))

(event EventInteractionEvent
  (Audio|PlaySoundatLocation "/Game/Audio/Door_Open.Door_Open" "0, 0, 0" "0, 0, 0" 1.0 1.0 0.0 0 0 0)
  (if (Variables|Default|GetFirstclose?)
    (Variables|Default|SetFirstclose? false)
    (bind _yaw (Timeline|Open%20Door ReverseFromEnd)
      (:Update
        (Transformation|SetRelativeRotation (Variables|Character|GetMesh) (Math|Rotator|MakeRotator 0.0 0.0 (* _yaw (Variables|Default|GetOpen%20Angle))) false false)))
    (elif (not (Variables|Default|GetOpen?))
      (Variables|Default|SetOpen? (not (Variables|Default|GetOpen?)))
      (Timeline|Open%20Door Reverse)
      (else
        (Variables|Default|SetOpen? (not (Variables|Default|GetOpen?)))
        (Timeline|Open%20Door Play)))))

(fn ConstructionScript
  (|CallParentFunction))