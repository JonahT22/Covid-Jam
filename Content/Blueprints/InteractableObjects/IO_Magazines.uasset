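; Interactable magazines prop with three meshes that is destroyed when its interaction event fires.
; On BeginPlay, each mesh gets one of three purple materials through nested random rolls, so the odds are uneven.
; While active, its interactable toggle shows or hides the interact text and switches custom depth rendering on all three meshes, presumably for highlighting.
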(event EventBeginPlay
  (bind _returnvalue (Math|Random|RandomInteger 3))
  (bind _returnvalue_2 (Math|Random|RandomInteger 3))
  (bind _returnvalue_3 (Math|Random|RandomInteger 3))
  (bind _mesh (Variables|Character|GetMesh))
  (bind _staticmesh (Variables|Default|GetStaticMesh))
  (bind _staticmesh1 (Variables|Default|GetStaticMesh1))
  (|CallParentFunction)
  (if (== _returnvalue 0)
    (Rendering|Material|SetMaterial _mesh 0 "/Game/Geometry/Materials/purple1.purple1")
    (elif (== _returnvalue 1)
      (Rendering|Material|SetMaterial _mesh 0 "/Game/Geometry/Materials/purple2.purple2")
      (else
        (Rendering|Material|SetMaterial _mesh 0 "/Game/Geometry/Materials/purple3.purple3"))))
  (if (== _returnvalue_2 0)
    (Rendering|Material|SetMaterial _staticmesh 0 "/Game/Geometry/Materials/purple1.purple1")
    (elif (== _returnvalue_2 1)
      (Rendering|Material|SetMaterial _staticmesh 0 "/Game/Geometry/Materials/purple2.purple2")
      (else
        (Rendering|Material|SetMaterial _staticmesh 0 "/Game/Geometry/Materials/purple3.purple3"))))
  (if (== _returnvalue_3 0)
    (Rendering|Material|SetMaterial _staticmesh1 0 "/Game/Geometry/Materials/purple1.purple1")
    (elif (== _returnvalue_3 1)
      (Rendering|Material|SetMaterial _staticmesh1 0 "/Game/Geometry/Materials/purple2.purple2")
      (else
        (Rendering|Material|SetMaterial _staticmesh1 0 "/Game/Geometry/Materials/purple3.purple3")))))

(event Collision|EventActorBeginOverlap
  (params (OtherActor :type Actor%20Object%20Reference)))

(event EventTick
  (params (DeltaSeconds :type Float%20%28single-precision%29)))

(event EventInteractionEvent
  (Actor|DestroyActor))

(fn ConstructionScript
  (|CallParentFunction))

(fn ChangeInteractable
  (params (Interactable? :type Boolean))
  (if (Variables|Default|GetAm%20Active?)
    (if Interactable?
      (Development|SetHiddeninGame (Variables|Default|GetInteract%20Text) false false)
      (Variables|Default|SetAm%20Interactable? true)
      (Rendering|SetRenderCustomDepth (Variables|Character|GetMesh) true)
      (else
        (Development|SetHiddeninGame (Variables|Default|GetInteract%20Text) true false)
        (Variables|Default|SetAm%20Interactable? false)
        (Rendering|SetRenderCustomDepth (Variables|Character|GetMesh) false)))))