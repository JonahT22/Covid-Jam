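; Interactable sofa that the player tidies to complete the first task (index 0).
; InteractionEvent runs CleanSofa, which plays a blanket-folding sound at world origin, swaps the mesh to the clean blanket and shifts it by a fixed offset.
; It queues a make-bed dialogue, deactivates the object, then queues a news popup dialogue before the task is checked off.
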(event Custom|CleanSofa
  (bind _mesh (Variables|Character|GetMesh))
  (bind _dialoguecontroller_ref (Variables|Default|GetDialogueController%20Ref))
  (Audio|PlaySoundatLocation "/Game/Audio/Fold_Blanket.Fold_Blanket" "0, 0, 0" "0, 0, 0" 1.0 1.0 0.0 0 0 0)
  (Components|StaticMesh|SetStaticMesh _mesh "/Game/Geometry/Meshes/ALL_clean_blanket.ALL_clean_blanket")
  (Transformation|AddRelativeLocation _mesh "-80.000000, 0,30.000000" false false)
  (Default|AddDialoguetoQueue _dialoguecontroller_ref "/Game/Blueprints/DialogueInteractions/ConversationSheets/Dialogue_Interactions_-_Make_Bed.Dialogue_Interactions_-_Make_Bed")
  (CallFunction|BecomeInactive)
  (Default|AddDialoguetoQueue _dialoguecontroller_ref "/Game/Blueprints/DialogueInteractions/ConversationSheets/Dialogue_Interactions_-_News_Popup.Dialogue_Interactions_-_News_Popup"))

(event EventBeginPlay
  (|CallParentFunction) ; This node is disabled and will not be called.\nDrag off pins to build functionality.
)

(event Collision|EventActorBeginOverlap
  (params (OtherActor :type Actor%20Object%20Reference)))

(event EventTick
  (params (DeltaSeconds :type Float%20%28single-precision%29)))

(event EventInteractionEvent
  (CallFunction|CleanSofa)
  (CallFunction|CheckOffTask))

(fn ConstructionScript
  (|CallParentFunction))