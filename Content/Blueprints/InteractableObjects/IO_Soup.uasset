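; IO_Soup is an interactable object that lets the player make soup.
; Interacting calls MakeSoup, which plays a bowl-clacking sound, swaps the mesh to a soup pot, nudges it upward and reveals the Bowl component.
; It then deactivates itself and spawns an active IO_SoupBowl pickup at a hardcoded world location with a "Pick Up Soup" prompt.
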(event Custom|MakeSoup
  (bind _mesh (Variables|Character|GetMesh))
  (Audio|PlaySoundatLocation "/Game/Audio/Bowls_Clacking.Bowls_Clacking" "0, 0, 0" "0, 0, 0" 1.0 1.0 0.0 0 0 0)
  (Components|StaticMesh|SetStaticMesh _mesh "/Game/Geometry/Meshes/ALL_souppot.ALL_souppot")
  (Transformation|AddRelativeLocation _mesh "0,0.000000,12.500000" false false)
  (Rendering|SetVisibility (Variables|Default|GetBowl) true false)
  (CallFunction|BecomeInactive)
  (Game|SpawnActorfromClass "/Game/Blueprints/InteractableObjects/IO_SoupBowl.IO_SoupBowl_C" (Math|Conversions|ToTransform(Vector) "-2200.000000,50.000000,220.000000") "AlwaysSpawn" 0 0 "Pick Up Soup" true 0))

(event EventBeginPlay
  (|CallParentFunction) ; This node is disabled and will not be called.\nDrag off pins to build functionality.
)

(event Collision|EventActorBeginOverlap
  (params (OtherActor :type Actor%20Object%20Reference)))

(event EventTick
  (params (DeltaSeconds :type Float%20%28single-precision%29)))

(event EventInteractionEvent
  (CallFunction|MakeSoup))

(fn ConstructionScript
  (|CallParentFunction))