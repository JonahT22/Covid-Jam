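; Interactable soup bowl that the player picks up, built on a parent interactable class.
; On BeginPlay it adds the make-lunch interaction dialogue sheet to its list.
; When interacted with, it hides its mesh, deactivates itself, notifies the player controller of the pickup and sends that dialogue sheet to the controller.
; It then activates every bedroom door actor in the level, with a leftover debug print for each.
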(event EventBeginPlay
  (|CallParentFunction)
  (Utilities|Array|Add (Variables|Default|GetDialogue%20Sheets) "/Game/Blueprints/DialogueInteractions/ConversationSheets/Dialogue_Interactions_-_M_Make_Lunch.Dialogue_Interactions_-_M_Make_Lunch"))

(event Collision|EventActorBeginOverlap
  (params (OtherActor :type Actor%20Object%20Reference)))

(event EventTick
  (params (DeltaSeconds :type Float%20%28single-precision%29)))

(event EventInteractionEvent
  (Rendering|SetVisibility (Variables|Character|GetMesh) false false)
  (CallFunction|BecomeInactive)
  (Default|PickedUpSoup (Variables|Default|GetPlayer%20Controller))
  (CallFunction|SendDialogueSheettoController)
  (bind _outactors (Actor|GetAllActorsOfClass "/Game/Blueprints/InteractableObjects/IO_BedroomDoor.IO_BedroomDoor_C"))
  (for _array_element _outactors
    (Default|BecomeActive _array_element)
    (Development|PrintString "door")))

(fn ConstructionScript
  (|CallParentFunction))