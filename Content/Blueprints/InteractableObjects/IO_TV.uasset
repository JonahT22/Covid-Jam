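; Interactable TV prop that shows text on an in-world screen widget.
; Its interaction event passes a hardcoded test line to AddTVText, which casts the TVText component's user widget to TVScreen and appends the text to its scroll box.
; BeginPlay and the construction script add no logic of their own, and a mesh material setter is left unconnected.
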(event Custom|Add%20TV%20text
  (params (New%20Text :type Text))
  ;[0.1719 0 1] Add text to widget
  (bind _astvscreen (Utilities|Casting|CastToTVScreen (UserInterface|GetUserWidgetObject (Variables|Default|GetTVText))))
  (Default|AddTexttoScreenScrollBox _astvscreen New%20Text))

(event EventBeginPlay
  (|CallParentFunction) ; This node is disabled and will not be called.\nDrag off pins to build functionality.
)

(event Collision|EventActorBeginOverlap
  (params (OtherActor :type Actor%20Object%20Reference)))

(event EventTick
  (params (DeltaSeconds :type Float%20%28single-precision%29)))

(event EventInteractionEvent
  (CallFunction|AddTVText "This is some test computer text that extends for an entire line until the line starts to wrap"))

(fn ConstructionScript
  (|CallParentFunction))