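; Base interactable object that the player can use when inside its capsule range and mousing over it.
; Overlap and mouse-over state together toggle the prompt widget and custom-depth rendering on the mesh while it is active.
; AcceptInput fires InteractionEvent, meant for child Blueprints to override.
; Helpers queue dialogue sheets and update the todo list, with both references auto-found at BeginPlay if unset.
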(event OnComponentBeginOverlap(Capsule)
  (params (OverlappedComponent :type Primitive%20Component%20Object%20Reference) (OtherActor :type Actor%20Object%20Reference) (OtherComp :type Primitive%20Component%20Object%20Reference) (OtherBodyIndex :type Integer) (bFromSweep :type Boolean) (SweepResult :type Hit%20Result%20Structure%20%28by%20ref%29))
  ;[0 1 0.8594] Begin/End overlap
  (if (== OtherActor (Variables|Default|GetPlayerCharacter))
    (Variables|Default|SetIn%20Range? true)
    (if (Variables|Default|GetMouse%20Over?)
      (CallFunction|ChangeInteractable true))))

(event OnComponentEndOverlap(Capsule)
  (params (OverlappedComponent :type Primitive%20Component%20Object%20Reference) (OtherActor :type Actor%20Object%20Reference) (OtherComp :type Primitive%20Component%20Object%20Reference) (OtherBodyIndex :type Integer))
  ;[0 1 0.8594] Begin/End overlap
  (if (== OtherActor (Variables|Default|GetPlayerCharacter))
    (Variables|Default|SetIn%20Range? false)
    (CallFunction|ChangeInteractable false)))

(event Custom|Interaction%20Event
  (Variables|Default|SetAm%20Active? false)
  (Development|SetHiddeninGame (Variables|Default|GetInteract%20Text) true false))

(event EventBeginPlay
  ;[1 0 0.375] get player character at start of game
  (CallFunction|SetInteractText)
  (bind _aschar_covid_character (Utilities|Casting|CastToChar_CovidCharacter (Game|GetPlayerCharacter 0)))
  (Variables|Default|SetPlayerCharacter _aschar_covid_character)
  (Variables|Default|SetPlayer%20Camera (Variables|/Game/Blueprints/Char_CovidCharacter.Char_CovidCharacter_C|GetFirstPersonCamera _aschar_covid_character))
  (bind _aspc_covid (Utilities|Casting|CastToPC_Covid (Game|GetPlayerController 0)))
  (Variables|Default|SetPlayer%20Controller _aspc_covid)
  (Utilities|FlowControl|Sequence
    (:then_0
      (Utilities|IsValid (Variables|Default|GetDialogueController%20Ref)
        (:Is%20Not%20Valid
          (bind _outactors (Actor|GetAllActorsOfClass "/Game/Blueprints/DialogueController.DialogueController_C"))
          (for _array_element _outactors
            (Variables|Default|SetDialogueController%20Ref _array_element))
          (Development|PrintString "WARNING: Dialogue controller ref not set in interactable object. Automatically setting dialogue controller ref..."))))
    (:then_1
      (Utilities|IsValid (Variables|Default|GetTodo%20List%20Ref)
        (:Is%20Not%20Valid
          (bind _outactors_2 (Actor|GetAllActorsOfClass "/Game/Blueprints/BP_Todo_List.BP_Todo_List_C"))
          (for _array_element_2 _outactors_2
            (Variables|Default|SetTodo%20List%20Ref _array_element_2))
          (Development|PrintString "WARNING: Todo list ref not set in interactable object. Automatically setting ref..."))))))

(fn ConstructionScript
  (Components|Capsule|SetCapsuleRadius (Variables|Default|GetCapsule) (Variables|Default|GetInteractionRadius) true))

(fn SetInteractText
  (bind _asinteractable_object_text (Utilities|Casting|CastToInteractableObjectText (UserInterface|GetUserWidgetObject (Variables|Default|GetInteract%20Text))))
  (Rendering|Components|TextRender|SetText (Variables|/Game/Blueprints/InteractableObjects/InteractableObjectText.InteractableObjectText_C|GetInteractionText _asinteractable_object_text) (Variables|Default|GetInteractionText)))

(fn ChangeInteractable
  (params (Interactable? :type Boolean))
  (if (Variables|Default|GetAm%20Active?)
    (if Interactable?
      (Development|SetHiddeninGame (Variables|Default|GetInteract%20Text) false false)
      (Variables|Default|SetAm%20Interactable? true)
      (Rendering|SetRenderCustomDepth (Variables|Default|GetMesh) true)
      (else
        (Development|SetHiddeninGame (Variables|Default|GetInteract%20Text) true false)
        (Variables|Default|SetAm%20Interactable? false)
        (Rendering|SetRenderCustomDepth (Variables|Default|GetMesh) false)))))

(fn BecomeInactive
  (Variables|Default|SetAm%20Active? false)
  (Variables|Default|SetAm%20Interactable? false)
  (Development|SetHiddeninGame (Variables|Default|GetInteract%20Text) true false))

(fn BeginMouseOver
  (Variables|Default|SetMouse%20Over? true)
  (if (Variables|Default|GetIn%20Range?)
    (CallFunction|ChangeInteractable true)))

(fn EndMouseOver
  (Variables|Default|SetMouse%20Over? false)
  (CallFunction|ChangeInteractable false))

(fn AcceptInput
  (if (Variables|Default|GetIn%20Range?)
    (if (Variables|Default|GetMouse%20Over?)
      (CallFunction|InteractionEvent))))

(fn SendDialogueSheettoController
  (params (Sheet%20index :type Integer))
  (bind _dialogue_sheets (Variables|Default|GetDialogue%20Sheets))
  (if (Utilities|Array|IsValidIndex _dialogue_sheets Sheet%20index)
    (Default|AddDialoguetoQueue (Variables|Default|GetDialogueController%20Ref) (Utilities|Array|Get(acopy) _dialogue_sheets Sheet%20index))
    (else
      (Development|PrintString "ERROR: Attempted to access invalid dialogue sheet in Interactable Object" true true "(R=0.000000,G=0.660000,B=1.000000,A=1.000000)" 2e+01))))

(fn CheckOffTask
  (params (Task%20Index :type Integer))
  (Default|CheckOffItem (Variables|Default|GetTodo%20List%20Ref) Task%20Index))

(fn AddStickytoTodoList
  (params (Sticky%20Number :type Integer))
  (Default|AddStickyNote (Variables|Default|GetTodo%20List%20Ref) Sticky%20Number))