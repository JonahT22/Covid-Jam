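; PC_Covid is the player controller that links a dialogue system to the gameplay UI.
; It creates the WB_GameplayUI widget on BeginPlay and relays phone texts, thoughts and timed prompts to it.
; Three dialogue input actions send the chosen prompt index to both the registered dialogue controller and the UI, provided that controller is valid.
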(event Custom|Send%20lines%20to%20phone
  (params (Line%20Text :type Text) (Speaker :type Enum_Speakers%20Enum :default "NewEnumerator0"))
  ;[0.8047 1 0] Send phone texts to gameplay UI
  (Default|AddPhoneText (Variables|Default|GetGameplay%20UI) Line%20Text Speaker))

(event Custom|Send%20prompts%20to%20Gameplay%20UI
  (params (Prompt%20lines :type Array%20of%20Texts) (Input%20time%20out :type Float%20%28single-precision%29))
  ;[1 0 0] Send prompts to screen
  (Default|SendPrompts (Variables|Default|GetGameplay%20UI) Prompt%20lines Input%20time%20out))

(event Custom|Send%20lines%20to%20Thoughts
  (params (New%20Text :type Text))
  ;[1 0 0.4453] Send thoughts to gameplay UI
  (Default|AddThoughtText (Variables|Default|GetGameplay%20UI) New%20Text))

(event EventBeginPlay
  ;[0.6641 1 0] Create gameplay UI widget
  (bind _returnvalue (UserInterface|CreateWidget "/Game/UI/WB_GameplayUI.WB_GameplayUI_C"))
  (bind _output_get (Variables|Default|SetGameplay%20UI _returnvalue))
  (UserInterface|Viewport|AddtoViewport _output_get 0))

(event Input|ActionEvents|InputActionDL_Input1
  (params (Key :type Key%20Structure :default "None"))
  (bind _dialogue_input_bp (Variables|Default|GetDialogue%20Input%20BP))
  ;[0 1 0.6016] Send dialogue inputs (2 options)
  (:Pressed
    (Variables|Default|SetChosen%20Prompt%20Index 1)
    (Utilities|IsValid _dialogue_input_bp
      (:Is%20Valid
        (Default|ReceiveInput _dialogue_input_bp (Variables|Default|GetChosen%20Prompt%20Index))
        (Default|ChoosePrompt (Variables|Default|GetGameplay%20UI) (Variables|Default|GetChosen%20Prompt%20Index))))))

(event Input|ActionEvents|InputActionDL_Input2
  (params (Key :type Key%20Structure :default "None"))
  (bind _dialogue_input_bp (Variables|Default|GetDialogue%20Input%20BP))
  ;[0 1 0.6016] Send dialogue inputs (2 options)
  (:Pressed
    (Variables|Default|SetChosen%20Prompt%20Index 2)
    (Utilities|IsValid _dialogue_input_bp
      (:Is%20Valid
        (Default|ReceiveInput _dialogue_input_bp (Variables|Default|GetChosen%20Prompt%20Index))
        (Default|ChoosePrompt (Variables|Default|GetGameplay%20UI) (Variables|Default|GetChosen%20Prompt%20Index))))))

(event Input|ActionEvents|InputActionDL_Input3
  (params (Key :type Key%20Structure :default "None"))
  (bind _dialogue_input_bp (Variables|Default|GetDialogue%20Input%20BP))
  ;[0 1 0.6016] Send dialogue inputs (2 options)
  (:Pressed
    (Variables|Default|SetChosen%20Prompt%20Index 3)
    (Utilities|IsValid _dialogue_input_bp
      (:Is%20Valid
        (Default|ReceiveInput _dialogue_input_bp (Variables|Default|GetChosen%20Prompt%20Index))
        (Default|ChoosePrompt (Variables|Default|GetGameplay%20UI) (Variables|Default|GetChosen%20Prompt%20Index))))))

(fn ConstructionScript)

(fn SetDialogueInputLocation
  (params (Dialogue%20Controller :type Dialogue%20Controller%20Object%20Reference))
  (Variables|Default|SetDialogue%20Input%20BP Dialogue%20Controller))