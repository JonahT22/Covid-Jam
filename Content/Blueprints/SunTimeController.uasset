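; Time-of-day controller that drives the directional sun, BP_GoodSky and time-triggered dialogue.
; Set and increment functions derive color and intensity goals by blending between day-phase keyframes, then an Ease timeline transitions sun and sky; morning, sunset and night presets skip dialogue and light checks.
; Point lights toggle past a threshold, gated by a dialogue flag, but their gathering code is unconnected.
; The second callout's condition is hard-wired true, making the first unreachable.
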(event Custom|Begin%20Moving%20sun
  ;[0 0.5781 1] Move sun and change directional light
  (Variables|Default|SetStart%20color (Rendering|Components|Light|GetLightColor (Variables|Default|GetSunlight%20Ref)))
  (Variables|Default|SetMoving%20sun? true)
  (Variables|Default|SetStart%20Intensity (Variables|/Script/Engine.LightComponentBase|GetIntensity (Variables|Default|GetSunlight%20Ref)))
  ;[0.5 1 0] Ease lighting to desired values
  (bind _alpha (Timeline|Ease PlayFromStart)
    (:Update
      (Rendering|Components|Light|SetLightColor (Variables|Default|GetSunlight%20Ref) (Math|Color|Lerp(LinearColor) (Variables|Default|GetStart%20color) (Variables|Default|GetColorGoal) _alpha) true)
      (Rendering|Components|Light|SetIntensity (Variables|Default|GetSunlight%20Ref) (Math|Float|Lerp (Variables|Default|GetStart%20Intensity) (Variables|Default|GetIntensity%20Goal) _alpha))
      (Variables|/Game/GoodSky/Blueprint/BP_GoodSky.BP_GoodSky_C|SetCustom%20Time%20of%20day (Variables|Default|GetGood%20Sky%20Ref) (Math|Float|%(Float) (+ (Math|Float|Lerp (Variables|Default|GetOldTimeOfDay) (Variables|Default|GetTimeOfDay) _alpha) 8.5) 24.0)))
    (:Finished
      (Variables|Default|SetMoving%20sun? false))))

(event EventBeginPlay
  ;[0.8516 0 1] Get light ref at start of game
  (Utilities|FlowControl|Sequence
    (:then_0
      ;;[0.4297 0 1] Check for directional light
      (Utilities|IsValid (Variables|Default|GetDirectional%20Light%20Ref)
        (:Is%20Valid
          _)
        (:Is%20Not%20Valid
          (Development|PrintString "WARNING: Directional light not set in suntime controller. Automatically setting...")
          (bind _outactors (Actor|GetAllActorsOfClass "/Script/Engine.DirectionalLight"))
          (for _array_element _outactors
            (Variables|Default|SetDirectional%20Light%20Ref _array_element))))
      (Variables|Default|SetSunlight%20Ref (Variables|/Script/Engine.Light|GetLightComponent (Variables|Default|GetDirectional%20Light%20Ref))))
    (:then_1
      ;;[0 0.1797 1] Check for good sky
      (Utilities|IsValid (Variables|Default|GetGood%20Sky%20Ref)
        (:Is%20Not%20Valid
          (Development|PrintString "WARNING: Good sky not set in suntime controller. Automatically setting...")
          (bind _outactors_2 (Actor|GetAllActorsOfClass "/Game/GoodSky/Blueprint/BP_GoodSky.BP_GoodSky_C"))
          (for _array_element_2 _outactors_2
            (Variables|Default|SetGood%20Sky%20Ref _array_element_2)))))
    (:then_2
      ;;[0.5938 0 1] check for dialogue controller
      (Utilities|IsValid (Variables|Default|GetDialogueController)
        (:Is%20Not%20Valid
          (Development|PrintString "WARNING: Dialogue controller not set in suntime controller. Automatically setting...")
          (bind _outactors_3 (Actor|GetAllActorsOfClass "/Game/Blueprints/DialogueController.DialogueController_C"))
          (for _array_element_3 _outactors_3
            (Variables|Default|SetDialogueController _array_element_3)))))
    (:then_3
      ;;[0.7578 1 0] Initialize sun from default time of day
      (CallFunction|SetSunandLights (Variables|Default|GetTimeOfDay)))))

(fn ConstructionScript)

(fn SetTimeOfDay
  (params (new%20time :type Float%20%28single-precision%29))
  (Variables|Default|SetOldTimeOfDay (Variables|Default|GetTimeOfDay))
  (bind _output_get (Variables|Default|SetTimeOfDay (Math|Float|Clamp(Float) new%20time 0.0 24.0)))
  (bind (_color _intensity) (CallFunction|TimetoColorandIntensity _output_get))
  (Variables|Default|SetColorGoal _color)
  (Variables|Default|SetIntensity%20Goal _intensity)
  (CallFunction|SetSunandLights new%20time)
  (CallFunction|CheckforDialogueTriggers (Variables|Default|GetTimeOfDay)))

(fn IncrementTimeOfDay
  (params (Time%20offset :type Float%20%28single-precision%29))
  (Variables|Default|SetOldTimeOfDay (Variables|Default|GetTimeOfDay))
  (bind _output_get (Variables|Default|SetTimeOfDay (Math|Float|Clamp(Float) (+ Time%20offset (Variables|Default|GetTimeOfDay)) 0.0 24.0)))
  (bind (_color _intensity) (CallFunction|TimetoColorandIntensity _output_get))
  (Variables|Default|SetColorGoal _color)
  (Variables|Default|SetIntensity%20Goal _intensity)
  (CallFunction|SetSunandLights (Variables|Default|GetTimeOfDay))
  (CallFunction|CheckforDialogueTriggers (Variables|Default|GetTimeOfDay)))

(fn TimetoColorandIntensity
  (params (Time :type Float%20%28single-precision%29))
  (bind _output_get (LocalVariables|SetL_Time Time))
  (if (>= _output_get (Variables|StaticVariables|GetMorning%20Time))
    (if (>= (LocalVariables|GetL_Time) (Variables|StaticVariables|GetMidafternoon%20Time))
      (if (>= (LocalVariables|GetL_Time) (Variables|StaticVariables|GetSunset%20Time))
        (if (>= (LocalVariables|GetL_Time) (Variables|StaticVariables|GetLate%20Sunset%20Time))
          (if (>= (LocalVariables|GetL_Time) (Variables|StaticVariables|GetNight%20Time))
            (LocalVariables|SetL_Color (Variables|StaticVariables|GetNight%20Color)) ; after night
            (else
              (LocalVariables|SetL_Color (Math|Color|Lerp(LinearColor) (Variables|StaticVariables|GetLate%20Sunset%20Color) (Variables|StaticVariables|GetNight%20Color) (/ (- (LocalVariables|GetL_Time) (Variables|StaticVariables|GetLate%20Sunset%20Time)) (- (Variables|StaticVariables|GetNight%20Time) (Variables|StaticVariables|GetLate%20Sunset%20Time))))) ; after late sunset
            ))
          (LocalVariables|SetL_Intensity (Math|Float|Lerp (Variables|StaticVariables|GetLate%20Sunset%20Intensity) (Variables|StaticVariables|GetNight%20Intensity) (/ (- (LocalVariables|GetL_Time) (Variables|StaticVariables|GetLate%20Sunset%20Time)) (- (Variables|StaticVariables|GetNight%20Time) (Variables|StaticVariables|GetLate%20Sunset%20Time)))))
          (else
            (LocalVariables|SetL_Color (Math|Color|Lerp(LinearColor) (Variables|StaticVariables|GetSunset%20Color) (Variables|StaticVariables|GetLate%20Sunset%20Color) (/ (- (LocalVariables|GetL_Time) (Variables|StaticVariables|GetSunset%20Time)) (- (Variables|StaticVariables|GetLate%20Sunset%20Time) (Variables|StaticVariables|GetSunset%20Time))))) ; Between sunset and late sunset
            (LocalVariables|SetL_Intensity (Math|Float|Lerp (Variables|StaticVariables|GetSunset%20Intensity) (Variables|StaticVariables|GetLate%20Sunset%20Intensity) (/ (- (LocalVariables|GetL_Time) (Variables|StaticVariables|GetSunset%20Time)) (- (Variables|StaticVariables|GetLate%20Sunset%20Time) (Variables|StaticVariables|GetSunset%20Time)))))))
        (else
          (LocalVariables|SetL_Color (Math|Color|Lerp(LinearColor) (Variables|StaticVariables|GetMidafternoon%20Color) (Variables|StaticVariables|GetSunset%20Color) (/ (- (LocalVariables|GetL_Time) (Variables|StaticVariables|GetMidafternoon%20Time)) (- (Variables|StaticVariables|GetSunset%20Time) (Variables|StaticVariables|GetMidafternoon%20Time))))) ; Between midafternoon and sunset
          (LocalVariables|SetL_Intensity (Math|Float|Lerp (Variables|StaticVariables|GetMidafternoon%20Intensity) (Variables|StaticVariables|GetSunset%20Intensity) (/ (- (LocalVariables|GetL_Time) (Variables|StaticVariables|GetMidafternoon%20Time)) (- (Variables|StaticVariables|GetSunset%20Time) (Variables|StaticVariables|GetMidafternoon%20Time)))))))
      (else
        (LocalVariables|SetL_Color (Math|Color|Lerp(LinearColor) (Variables|StaticVariables|GetMorning%20Color) (Variables|StaticVariables|GetMidafternoon%20Color) (/ (- (LocalVariables|GetL_Time) (Variables|StaticVariables|GetMorning%20Time)) (- (Variables|StaticVariables|GetMidafternoon%20Time) (Variables|StaticVariables|GetMorning%20Time))))) ; Between morning and midafternoon
        (LocalVariables|SetL_Intensity (Math|Float|Lerp (Variables|StaticVariables|GetMorning%20Intensity) (Variables|StaticVariables|GetMidafternoon%20Intensity) (/ (- (LocalVariables|GetL_Time) (Variables|StaticVariables|GetMorning%20Time)) (- (Variables|StaticVariables|GetMidafternoon%20Time) (Variables|StaticVariables|GetMorning%20Time)))))))
    (else
      (LocalVariables|SetL_Color (Math|Color|Lerp(LinearColor) (Variables|StaticVariables|GetNight%20Color) (Variables|StaticVariables|GetMorning%20Color) (/ (LocalVariables|GetL_Time) (Variables|StaticVariables|GetMorning%20Time)))) ; Less than morningtime
      (LocalVariables|SetL_Intensity (Math|Float|Lerp (Variables|StaticVariables|GetNight%20Intensity) (Variables|StaticVariables|GetMorning%20Intensity) (/ (LocalVariables|GetL_Time) (Variables|StaticVariables|GetMorning%20Time))))))
  (return (LocalVariables|GetL_Color) (LocalVariables|GetL_Intensity)))

(fn SetTimetoMorning
  (bind _output_get (Variables|Default|SetTimeOfDay (Variables|StaticVariables|GetMorning%20Time)))
  (bind (_color _intensity) (CallFunction|TimetoColorandIntensity _output_get))
  (Variables|Default|SetColorGoal _color)
  (Variables|Default|SetIntensity%20Goal _intensity)
  (CallFunction|BeginMovingSun))

(fn SetTimetoSunset
  (bind _output_get (Variables|Default|SetTimeOfDay (Variables|StaticVariables|GetSunset%20Time)))
  (bind (_color _intensity) (CallFunction|TimetoColorandIntensity _output_get))
  (Variables|Default|SetColorGoal _color)
  (Variables|Default|SetIntensity%20Goal _intensity)
  (CallFunction|BeginMovingSun))

(fn SetTimetoNight
  (bind _output_get (Variables|Default|SetTimeOfDay (Variables|StaticVariables|GetNight%20Time)))
  (bind (_color _intensity) (CallFunction|TimetoColorandIntensity _output_get))
  (Variables|Default|SetColorGoal _color)
  (Variables|Default|SetIntensity%20Goal _intensity)
  (CallFunction|BeginMovingSun))

(fn SetSunandLights
  (params (Time :type Float%20%28single-precision%29))
  (Development|PrintString (Utilities|String|ToString(Text) (Utilities|Text|FormatText "current time: {time}" (Utilities|Text|ToText(String) (Utilities|String|ToString(Float) Time)))) true true "(R=0.000000,G=0.660000,B=1.000000,A=1.000000)" 1e+01)
  (CallFunction|BeginMovingSun)
  (if (< Time 11.0)
    (Development|PrintString "WARNING: Setting time below 11 results in bad lighting conditions"))
  ;[1 0.8203 0] Should lights be on? Are they?
  (if (> Time (Variables|Default|GetLightsOnTime))
    (if (not (Variables|Default|GetLights%20on?))
      (if (Variables|Default|GetLights%20on%20dialogue%20played)
        (Variables|Default|SetLights%20on? true)
        (for _array_element (Variables|Default|GetPointLights) :!label _label
          (Rendering|SetActorHiddenInGame _array_element (not (Variables|Default|GetLights%20on?))))
        (Development|PrintString (Utilities|String|ToString(Boolean) (Variables|Default|GetLights%20on?)))))
    (elif (Variables|Default|GetLights%20on?)
      (Variables|Default|SetLights%20on? false)
      (goto _label))))

(fn TurnonLightsfromDialogue)

(fn CheckforDialogueTriggers
  (params (Time :type Float%20%28single-precision%29))
  (if (> Time (Variables|DialogueTriggers|GetEnd%20of%20day%20time))
    (Default|AddDialoguetoQueue (Variables|Default|GetDialogueController) (Variables|DialogueTriggers|GetEnd%20of%20day%20table))
    (elif (> Time (Variables|DialogueTriggers|Gettime%20callout%203%20time))
      (Default|AddDialoguetoQueue (Variables|Default|GetDialogueController) (Variables|DialogueTriggers|GetCallout%203%20table))
      (elif true
        (Default|AddDialoguetoQueue (Variables|Default|GetDialogueController) (Variables|DialogueTriggers|GetCallout%202%20table))
        (elif (> Time (Variables|DialogueTriggers|GetTime%20Callout%201%20Time))
          (Default|AddDialoguetoQueue (Variables|Default|GetDialogueController) (Variables|DialogueTriggers|GetCallout%201%20table)))))))