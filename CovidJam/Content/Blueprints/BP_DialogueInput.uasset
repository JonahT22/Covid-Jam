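; BP_DialogueInput is a dialogue choice point that lets the player pick which monologue plays next.
; On activation it prints numbered prompts to the debug log, the only destination handled, and registers itself with PC_Covid as the input location.
; A received one-based index, if in range while waiting, activates the matching next sequence's monologue and stops waiting.
; The construction script shows the editor name on a text label.
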(event Custom|Activate%20Input
  ;[1 1 1] Start waiting for player input and print prompts
  (CallFunction|SendInputPromptstoDestination)
  (bind _aspc_covid (Utilities|Casting|CastToPC_Covid (Game|GetPlayerController 0)))
  (Default|SetDialogueInputLocation _aspc_covid self)
  (Variables|Default|SetWaiting%20for%20input? true))

(event Custom|Receive%20Input
  (params (Input%20Index :type Integer))
  ;[1 1 1] Activate monologue from input
  (if (Math|Boolean|ANDBoolean (Variables|Default|GetWaiting%20for%20input?) (>= Input%20Index 1) (<= Input%20Index (Utilities|Array|Length (Variables|Default|GetNextSequences))))
    (Default|ActivateMonologue (Utilities|Array|Get(acopy) (Variables|Default|GetNextSequences) (- Input%20Index 1)))
    (Variables|Default|SetWaiting%20for%20input? false)))

(fn ConstructionScript
  (Rendering|Components|TextRender|SetText (Variables|Default|GetName) (Variables|In-EditorName|GetEditorName)))

(fn SendInputPromptstoDestination
  (switch Utilities|FlowControl|Switch|SwitchonEnum_Destinations (Variables|Default|GetDestination)
    (:NewEnumerator0
      (for (_array_element _array_index) (Variables|Default|GetInput%20Prompts)
        (Development|PrintString (Utilities|String|ToString(Text) (Utilities|Text|FormatText "{number}. {text}" (Utilities|Text|ToText(Integer) (+ _array_index 1)) _array_element)) true true "(R=0.967059,G=0.980951,B=1.000000,A=1.000000)" 1e+01)))))