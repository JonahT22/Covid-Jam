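; Base dialogue controller that plays a branching conversation from a data table to the player's phone or debug log.
; A self-calling RepeatLoop event steps through numbered rows, allowing delays between lines and following Goto jumps.
; Input rows gather prompts for the gameplay UI via PC_Covid, then wait for a choice, with Tick selecting the last prompt on timeout.
; Event rows trigger two custom events intended for child Blueprints to override.
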(event Custom|Activate%20Dialogue%20Controller
  ;[1 0.4688 0] Initialize loop
  (if (not (Variables|Default|GetIs%20already%20active))
    (Variables|Default|SetIs%20already%20active true)
    (Variables|Default|SetCurrLineNum 1)
    ;[1 0 0.5625] Get Data table line
    (bind _returnvalue (Utilities|GetDataTableRow (Variables|Default|GetDialogueTable) (Utilities|String|StringToName (Utilities|String|ToString(Integer) (Variables|Default|GetCurrLineNum))))
      (:then
        (Variables|Default|SetCurrLineData _returnvalue)
        ;[0.1016 0 1] Check Goto value
        (if (== 0 (.goto (Variables|Default|GetCurrLineData))) ; If goto has a value, go to that, else increment
          (Math|Integer|IncrementInt (Variables|Default|GetCurrLineNum)
            (:%20%20
              _))
          (else
            (Variables|Default|SetCurrLineNum (.goto (Variables|Default|GetCurrLineData)))))
        ;[0.4766 1 0] Check line type
        (switch Utilities|FlowControl|Switch|SwitchonEnum_LineTypes (.type (Variables|Default|GetCurrLineData))
          (:NewEnumerator0
            ;[0.7109 0 1] Handle Outputting lines
            (Utilities|FlowControl|Delay (.predelay (Variables|Default|GetCurrLineData)))
            (CallFunction|SendLinetoDestination (.text (Variables|Default|GetCurrLineData)) (.destination (Variables|Default|GetCurrLineData)) (.speaker (Variables|Default|GetCurrLineData)))
            (Utilities|FlowControl|Delay (.postdelay (Variables|Default|GetCurrLineData)))
            (CallFunction|RepeatLoop))
          (:NewEnumerator1
            ;[0.1719 1 0] Handle Prompt type input error
            (Development|PrintString (Utilities|String|ToString(Text) (Utilities|Text|FormatText "ERROR: Prompt sent to output on row {row} " (Utilities|Text|ToText(String) (Utilities|String|ToString(Integer) (Variables|Default|GetCurrLineNum))))) true true "(R=0.000000,G=0.660000,B=1.000000,A=1.000000)" 2e+01))
          (:NewEnumerator2
            ;[0.125 1 0] Read the next few prompt lines until End input detected then break out of loop
            (CallFunction|ReadPrompts (Variables|Default|GetCurrLineNum)) ; Note: Curr line already incremented, starting line is 1st prompt
            (CallFunction|SendInputPrompts)
            (bind _aspc_covid (Utilities|Casting|CastToPC_Covid (Game|GetPlayerController 0)))
            (Default|SetDialogueInputLocation _aspc_covid self)
            (CallFunction|StartWaitingforInput))
          (:NewEnumerator3
            ;[0.1719 1 0] Handle End Input type error
            (Development|PrintString (Utilities|String|ToString(Text) (Utilities|Text|FormatText "ERROR: End of input sent to output on row {row} " (Utilities|Text|ToText(String) (Utilities|String|ToString(Integer) (Variables|Default|GetCurrLineNum))))) true true "(R=0.000000,G=0.660000,B=1.000000,A=1.000000)" 2e+01))
          (:NewEnumerator5
            ;[0.4531 1 0] Set up hooks for 2 custom events to be specified in child BPs
            (if (Utilities|Enum|Equal(Enum) (Utilities|String|ToString(Text) (.text (Variables|Default|GetCurrLineData))) "Event1")
              (CallFunction|CustomEvent1)
              (CallFunction|RepeatLoop :!label _label)
              (elif (Utilities|Enum|Equal(Enum) (Utilities|String|ToString(Text) (.text (Variables|Default|GetCurrLineData))) "Event2")
                (CallFunction|CustomEvent2)
                (goto _label))))
          (:NewEnumerator4
            (Development|PrintString "EOF Reached")
            (Variables|Default|SetIs%20already%20active false))))
      (:RowNotFound
        (Development|PrintString (Utilities|String|ToString(Text) (Utilities|Text|FormatText "ERROR: row {row} not found" (Utilities|Text|ToText(String) (Utilities|String|ToString(Integer) (Variables|Default|GetCurrLineNum))))) true true "(R=0.000000,G=0.660000,B=1.000000,A=1.000000)" 2e+01)))))

(event Custom|Receive%20Input
  (params (Input%20index :type Integer))
  ;[1 0 0.1406] Get input, resume reading dialogue sequence
  (if (Math|Boolean|ANDBoolean (Variables|Default|GetWaiting%20for%20input?) (>= Input%20index 1) (<= (- Input%20index 1) (Utilities|Array|Length (Variables|Prompts|GetPromptGotos))))
    (Variables|Default|SetCurrLineNum (Utilities|Array|Get(acopy) (Variables|Prompts|GetPromptGotos) (- Input%20index 1)))
    (Variables|Default|SetWaiting%20for%20Input? false)
    (CallFunction|RepeatLoop)))

(event Custom|CustomEvent1
  ;[0.1719 0 1] Custom events
  (Development|PrintString "Event1 Called"))

(event Custom|Repeat%20Loop
  ;[1 0.4688 0] Initialize loop
  ;[1 0 0.5625] Get Data table line
  (bind _returnvalue (Utilities|GetDataTableRow (Variables|Default|GetDialogueTable) (Utilities|String|StringToName (Utilities|String|ToString(Integer) (Variables|Default|GetCurrLineNum))))
    (:then
      (Variables|Default|SetCurrLineData _returnvalue)
      ;[0.1016 0 1] Check Goto value
      (if (== 0 (.goto (Variables|Default|GetCurrLineData))) ; If goto has a value, go to that, else increment
        (Math|Integer|IncrementInt (Variables|Default|GetCurrLineNum)
          (:%20%20
            _))
        (else
          (Variables|Default|SetCurrLineNum (.goto (Variables|Default|GetCurrLineData)))))
      ;[0.4766 1 0] Check line type
      (switch Utilities|FlowControl|Switch|SwitchonEnum_LineTypes (.type (Variables|Default|GetCurrLineData))
        (:NewEnumerator0
          ;[0.7109 0 1] Handle Outputting lines
          (Utilities|FlowControl|Delay (.predelay (Variables|Default|GetCurrLineData)))
          (CallFunction|SendLinetoDestination (.text (Variables|Default|GetCurrLineData)) (.destination (Variables|Default|GetCurrLineData)) (.speaker (Variables|Default|GetCurrLineData)))
          (Utilities|FlowControl|Delay (.postdelay (Variables|Default|GetCurrLineData)))
          (CallFunction|RepeatLoop))
        (:NewEnumerator1
          ;[0.1719 1 0] Handle Prompt type input error
          (Development|PrintString (Utilities|String|ToString(Text) (Utilities|Text|FormatText "ERROR: Prompt sent to output on row {row} " (Utilities|Text|ToText(String) (Utilities|String|ToString(Integer) (Variables|Default|GetCurrLineNum))))) true true "(R=0.000000,G=0.660000,B=1.000000,A=1.000000)" 2e+01))
        (:NewEnumerator2
          ;[0.125 1 0] Read the next few prompt lines until End input detected then break out of loop
          (CallFunction|ReadPrompts (Variables|Default|GetCurrLineNum)) ; Note: Curr line already incremented, starting line is 1st prompt
          (CallFunction|SendInputPrompts)
          (bind _aspc_covid (Utilities|Casting|CastToPC_Covid (Game|GetPlayerController 0)))
          (Default|SetDialogueInputLocation _aspc_covid self)
          (CallFunction|StartWaitingforInput))
        (:NewEnumerator3
          ;[0.1719 1 0] Handle End Input type error
          (Development|PrintString (Utilities|String|ToString(Text) (Utilities|Text|FormatText "ERROR: End of input sent to output on row {row} " (Utilities|Text|ToText(String) (Utilities|String|ToString(Integer) (Variables|Default|GetCurrLineNum))))) true true "(R=0.000000,G=0.660000,B=1.000000,A=1.000000)" 2e+01))
        (:NewEnumerator5
          ;[0.4531 1 0] Set up hooks for 2 custom events to be specified in child BPs
          (if (Utilities|Enum|Equal(Enum) (Utilities|String|ToString(Text) (.text (Variables|Default|GetCurrLineData))) "Event1")
            (CallFunction|CustomEvent1)
            (CallFunction|RepeatLoop :!label _label)
            (elif (Utilities|Enum|Equal(Enum) (Utilities|String|ToString(Text) (.text (Variables|Default|GetCurrLineData))) "Event2")
              (CallFunction|CustomEvent2)
              (goto _label))))
        (:NewEnumerator4
          (Development|PrintString "EOF Reached")
          (Variables|Default|SetIs%20already%20active false))))
    (:RowNotFound
      (Development|PrintString (Utilities|String|ToString(Text) (Utilities|Text|FormatText "ERROR: row {row} not found" (Utilities|Text|ToText(String) (Utilities|String|ToString(Integer) (Variables|Default|GetCurrLineNum))))) true true "(R=0.000000,G=0.660000,B=1.000000,A=1.000000)" 2e+01))))

(event Custom|Start%20Waiting%20for%20Input
  ;[1 0 0.4922] Start waiting for input
  (Variables|Default|SetInputTimeCounter 0.0)
  (Variables|Default|SetWaiting%20for%20Input? true))

(event Custom|CustomEvent2
  ;[0.1719 0 1] Custom events
  (Development|PrintString "Event2 Called"))

(event EventBeginPlay
  ;[1 0.9844 0] Get character and controller on beginplay
  (bind _aschar_covid_character (Utilities|Casting|CastToChar_CovidCharacter (Game|GetPlayerCharacter 0)))
  (Variables|Default|SetPlayerCharacter _aschar_covid_character)
  (bind _aspc_covid (Utilities|Casting|CastToPC_Covid (Game|GetPlayerController 0)))
  (Variables|Default|SetPlayerController _aspc_covid))

(event EventTick
  (params (DeltaSeconds :type Float%20%28single-precision%29))
  (bind _promptgotos (Variables|Prompts|GetPromptGotos))
  (bind _returnvalue (Utilities|Array|Length _promptgotos))
  ;[0 1 0.7188] Count down input timer, call last prompt otherwise
  (if (Variables|Default|GetWaiting%20for%20Input?)
    (if (> (Variables|Default|GetInputTimeCounter) (Variables|Default|GetInputTimeOut))
      ;[0.8281 0 1] Use the final prompt
      (Variables|Default|SetCurrLineNum (Utilities|Array|Get(acopy) _promptgotos (- _returnvalue 1)))
      (Variables|Default|SetWaiting%20for%20Input? false)
      (Default|ChoosePrompt (Variables|/Game/Blueprints/PC_Covid.PC_Covid_C|GetGameplay%20UI (Variables|Default|GetPlayerController)) _returnvalue)
      (CallFunction|RepeatLoop)
      (else
        (Variables|Default|SetInputTimeCounter (+ DeltaSeconds (Variables|Default|GetInputTimeCounter)))))))

(fn ConstructionScript)

(fn SendLinetoDestination
  (params (Line%20text :type Text) (Destination :type Enum_Destinations%20Enum :default "NewEnumerator0") (Speaker :type Enum_Speakers%20Enum :default "NewEnumerator0"))
  (LocalVariables|SetL_Text Line%20text)
  (LocalVariables|SetL_Speaker Speaker)
  (switch Utilities|FlowControl|Switch|SwitchonEnum_Destinations Destination
    (:NewEnumerator0
      ;[1 0.2109 0] Debug
      (switch Utilities|FlowControl|Switch|SwitchonEnum_Speakers (LocalVariables|GetL_Speaker)
        (:NewEnumerator0
          (Development|PrintString (Utilities|String|ToString(Text) (LocalVariables|GetL_Text)) true true "(R=0.000000,G=0.660000,B=1.000000,A=1.000000)" 1e+01))
        (:NewEnumerator1
          (Development|PrintString (Utilities|String|ToString(Text) (LocalVariables|GetL_Text)) true true "(R=1.000000,G=0.060419,B=0.120146,A=1.000000)" 1e+01))))
    (:NewEnumerator1
      ;[1 0.5156 0] Phone
      (Default|SendLinestoPhone (Variables|Default|GetPlayerController) (LocalVariables|GetL_Text) (LocalVariables|GetL_Speaker)))))

(fn SendInputPrompts
  (Default|SendPromptstoGameplayUI (Variables|Default|GetPlayerController) (Variables|Prompts|GetPromptsArray) (Variables|Default|GetInputTimeOut)))

(fn ReadPrompts
  (params (Starting%20Line :type Integer))
  (LocalVariables|SetLocal_CurrLine Starting%20Line)
  (Utilities|Array|Clear (Variables|Prompts|GetPromptsArray))
  (Utilities|Array|Clear (Variables|Prompts|GetPromptGotos))
  (while (not (LocalVariables|GetEndInput%20Reached?))
    (Utilities|FlowControl|Sequence
      (:then_0
        (bind _returnvalue (Utilities|GetDataTableRow (Variables|Default|GetDialogueTable) (Utilities|String|StringToName (Utilities|String|ToString(Integer) (LocalVariables|GetLocal_CurrLine))))
          (:then
            (switch Utilities|FlowControl|Switch|SwitchonEnum_LineTypes (.Type (Utilities|Struct|BreakStruct_LineData _returnvalue))
              (:NewEnumerator0
                ;[0.1719 1 0] Handle Input order error
                (Development|PrintString (Utilities|String|ToString(Text) (Utilities|Text|FormatText "ERROR: Encountered non-prompt/endinput while reading prompts on row {row} " (Utilities|Text|ToText(String) (Utilities|String|ToString(Integer) (Variables|Default|GetCurrLineNum))))) true true "(R=0.000000,G=0.660000,B=1.000000,A=1.000000)" 2e+01 :!label _label))
              (:NewEnumerator1
                ;[0 1 0.1328] Add prompts to array until end input reached
                (Utilities|Array|Add (Variables|Prompts|GetPromptsArray) (.Text (Utilities|Struct|BreakStruct_LineData _returnvalue)))
                (Utilities|Array|Add (Variables|Prompts|GetPromptGotos) (.Goto (Utilities|Struct|BreakStruct_LineData _returnvalue))))
              (:NewEnumerator2
                (goto _label))
              (:NewEnumerator3
                (LocalVariables|SetEndInput%20Reached? true))
              (:NewEnumerator4
                (goto _label))))))
      (:then_1
        (Math|Integer|IncrementInt (LocalVariables|GetLocal_CurrLine))))))