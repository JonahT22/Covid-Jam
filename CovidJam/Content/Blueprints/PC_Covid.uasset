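; PC_Covid, apparently a player controller, forwards dialogue choice input to a dialogue controller.
; SetDialogueInputLocation stores the target controller in DialogueInputBP.
; The DL_Input1 and DL_Input2 press actions check that the reference is valid, then call its ReceiveInput with the matching option number.
; Logic for a third option exists but is not connected to any event.
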(event EventBeginPlay)

(event EventTick
  (params (DeltaSeconds :type Float%20%28single-precision%29)))

(event Input|ActionEvents|InputActionDL_Input1
  (params (Key :type Key%20Structure :default "None"))
  (bind _dialogue_input_bp (Variables|Default|GetDialogue%20Input%20BP))
  ;[0 1 0.6016] Send dialogue inputs (2 options)
  (:Pressed
    (Utilities|IsValid _dialogue_input_bp
      (:Is%20Valid
        (Default|ReceiveInput _dialogue_input_bp 1)))))

(event Input|ActionEvents|InputActionDL_Input2
  (params (Key :type Key%20Structure :default "None"))
  (bind _dialogue_input_bp (Variables|Default|GetDialogue%20Input%20BP))
  ;[0 1 0.6016] Send dialogue inputs (2 options)
  (:Pressed
    (Utilities|IsValid _dialogue_input_bp
      (:Is%20Valid
        (Default|ReceiveInput _dialogue_input_bp 2)))))

(event Input|ActionEvents|InputActionDL_Input3
  (params (Key :type Key%20Structure :default "None"))
  ;[0 1 0.6016] Send dialogue inputs (2 options)
)

(fn ConstructionScript)

(fn SetDialogueInputLocation
  (params (Dialogue%20Controller :type Dialogue%20Controller%20Object%20Reference))
  (Variables|Default|SetDialogue%20Input%20BP Dialogue%20Controller))